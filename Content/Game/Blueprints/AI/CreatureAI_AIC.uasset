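; AI controller for creatures that runs Creature_BT and decides whether an animal reacts Friendly, Curious or Aggresive on seeing the player.
; Sight updates write the player and a run-away point to the blackboard.
; A random roll against species thresholds, shifted by the player's right-hand item, sets the reaction and emotion sprite, then resets thresholds to base variables.
; It also handles the grazeable flag and eating grass.
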(event `self.ReceiveBeginPlay`
  (`self.RunBehaviorTree` self "/Game/Game/Blueprints/AI/Creature_BT.Creature_BT")
  (`self.CheckAnimal`))

(event `self.Detection.OnTargetPerceptionUpdated`
  (params (Actor :type "Actor Object Reference") (Stimulus :type "AIStimulus Structure"))
  (bind (_age _expirationage _strength _stimuluslocation _receiverlocation _tag _bsuccessfullysensed) (break `AIStimulus` Stimulus))
  (bind _returnvalue (`GameplayStatics.GetPlayerCharacter` 0))
  (bind _returnvalue_2 (`self.K2_GetActorLocation` self))
  (bind _returnvalue_3 (`AIBlueprintHelperLibrary.GetBlackboard` self))
  ; Makes sure the animal has SEEN something
  (bind _returnvalue_4 (`AIPerceptionSystem.GetSenseClassForStimulus` Stimulus))
  (if (== _returnvalue_4 "/Script/AIModule.AISense_Sight")
    (if (== Actor _returnvalue)
      (`BlackboardComponent.SetValueAsObject` _returnvalue_3 "PlayerCharacter" (`KismetMathLibrary.SelectObject` _returnvalue null _bsuccessfullysensed))
      (`BlackboardComponent.SetValueAsVector` _returnvalue_3 "RunAwayLocation" (+ (* (`KismetMathLibrary.GetDirectionUnitVector` _returnvalue_2 _stimuluslocation) -200) _returnvalue_2))
      (if _bsuccessfullysensed
        ; Add the player's items modifier and generate a reaction
        (bind (_item _found) (`self.GetPlayerHeldItem` (`GameplayStatics.GetPlayerController` 0)))
        (if _found
          (`self.Add Item Modifier` (`/Game/Game/Blueprints/Items/BP_ItemObject.ReactionModifier` _item) (`/Game/Game/Blueprints/Items/BP_ItemObject.ReactionModified` _item)))
        (`self.GenerateRandomReaction`)
        (else
          ; if player has left range, hide the emotion indicator
          (`self.SetEmotionSprite` null))))))

(event `GenerateRandomReaction`
  (bind _returnvalue (`KismetMathLibrary.RandomInteger` 100))
  ; Determines what the animals reaction will be based on a random number
  (if (>= _returnvalue (`self.FriendlyValue`))
    (set `self.Reaction` "Friendly")
    (`self.SetEmotionSprite` "/Game/Game/Art/Ai_Sprites/emotionSprites1.emotionSprites1")
    (elif (<= _returnvalue (`self.AggresiveValue`))
      (set `self.Reaction` "Aggresive")
      (`self.SetEmotionSprite` "/Game/Game/Art/Ai_Sprites/emotionSprites3.emotionSprites3")
      (else
        (set `self.Reaction` "Curious")
        (`self.SetEmotionSprite` "/Game/Game/Art/Ai_Sprites/emotionSprites2.emotionSprites2"))))
  ; Sends this value to the behaviour tree to actually use it
  (`BlackboardComponent.SetValueAsString` (`AIBlueprintHelperLibrary.GetBlackboard` self) "Reaction" (`self.Reaction`))
  ; and resets the friendly and aggresive values back to the base
  (set `self.FriendlyValue` (`self.BaseFriendly`))
  (set `self.AggresiveValue` (`self.BaseAggre`)))

(event `Add Item Modifier`
  (params (Value :type Integer) (ReactionMod :type String))
  ; Goes through and adds a temporary value to the reaction check if the player's held item effects it
  (if (`KismetStringLibrary.EqualEqual_StrStr` ReactionMod "Friendly")
    (set `self.FriendlyValue` (- (`self.FriendlyValue`) Value))
    (elif (`KismetStringLibrary.EqualEqual_StrStr` ReactionMod "Curious")
      (set `self.FriendlyValue` (+ (`self.FriendlyValue`) Value))
      (set `self.AggresiveValue` (- (`self.AggresiveValue`) Value))
      (elif (`KismetStringLibrary.EqualEqual_StrStr` ReactionMod "Aggresive")
        (set `self.AggresiveValue` (+ (`self.AggresiveValue`) Value))))))

(event `CheckAnimal`
  (bind _returnvalue (`self.GetParentActor`))
  ; Changes the base values for how an animal will react based on which animal it is
  (cast `/Game/Game/Blueprints/AI/Pig_Creature/Pig_Creature_BP` _returnvalue
    (:`then`
      (set `self.FriendlyValue` 50)
      (set `self.AggresiveValue` 10))
    (:`CastFailed`
      (cast `/Game/Game/Blueprints/AI/Bird_Creature/Bird_Creature_BP` _returnvalue)
      (set `self.FriendlyValue` 75)
      (set `self.AggresiveValue` 25))))

(event `SetIsGrazeable`
  (params (Value :type Boolean))
  (bind _output_get (set `self.isGrazing` Value))
  (`BlackboardComponent.SetValueAsBool` (`AIBlueprintHelperLibrary.GetBlackboard` self) "IsGrazeable" _output_get))

(event `EatGrass`
  (bind _ascreature_bp (cast `/Game/Game/Blueprints/AI/Creature_BP` (`self.K2_GetPawn`)))
  (`/Game/Game/Blueprints/AI/Creature_BP.EatTileBelow` _ascreature_bp)
  (`self.SetIsGrazeable` false))

(fn `GetPlayerHeldItem`
  (params (Player :type "PlayerController Object Reference"))
  (returns (Item :type "/Game/Game/Blueprints/Items/BP_ItemObject Object Reference") (Found :type Boolean))
  (bind _asbp_platforming_character (cast `/Game/Unreal/Variant_Platforming/Blueprints/BP_PlatformingCharacter` (`self.K2_GetPawn` Player))
    (:`then`
      (bind (_item _world_item _found_) (`/Game/Game/Blueprints/Equipment/BPC_EquipmentComponent.GetEquipmentInSlot` (`/Game/Unreal/Variant_Platforming/Blueprints/BP_PlatformingCharacter.BPC_EquipmentComponent` _asbp_platforming_character) (struct :`TagName` "Equipment.RightHand")))
      (return _item _found_))
    (:`CastFailed`
      (`KismetSystemLibrary.PrintString` "okay player issue")
      (return null false))))

(fn `SetBlockBelow`)

(fn `SetEmotionSprite`
  (params (NewParam :type "Texture2D Object Reference"))
  (bind _ascreature_bp (cast `/Game/Game/Blueprints/AI/Creature_BP` (`self.K2_GetPawn`)))
  (`BillboardComponent.SetSprite` (`/Game/Game/Blueprints/AI/Creature_BP.CurrentEmotion` _ascreature_bp) NewParam))

(fn `TakePlayerHeldItem`
  (params (Player :type "PlayerController Object Reference"))
  (bind _asbp_platforming_character (cast `/Game/Unreal/Variant_Platforming/Blueprints/BP_PlatformingCharacter` (`self.K2_GetPawn` Player)))
  (bind _success (`/Game/Game/Blueprints/Inventory/BPC_InventoryComponent.RemoveItemAtCoordinate` (`/Game/Game/Blueprints/Equipment/BPC_EquipmentComponent.GetInventory` (`/Game/Unreal/Variant_Platforming/Blueprints/BP_PlatformingCharacter.BPC_EquipmentComponent` _asbp_platforming_character)) (make `/Game/Game/Blueprints/Inventory/FItemCoordinate` 0)))
  (`KismetSystemLibrary.PrintString` (`KismetStringLibrary.Conv_BoolToString` _success)))

(fn `UserConstructionScript`)