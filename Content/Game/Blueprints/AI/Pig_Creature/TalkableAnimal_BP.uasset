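; Talkable animal AI Blueprint that shows dialogue and hands the player a simple item quest.
; A detector overlap toggles the ShopCreature_AIC popup and sets the player controller's NearbyChar, hiding the dialogue box on exit.
; Talk shows a random basic line if the player has a quest; otherwise it appends Carrots or Wheat to a random prompt and sets HasQuest.
; The dialogue widget is created hidden on BeginPlay.
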(event `self.ReceiveBeginPlay`
  (`parent.ReceiveBeginPlay`)
  (bind _asbp_player_controller (cast `/Game/Game/Blueprints/Core/BP_PlayerController` (`GameplayStatics.GetPlayerController` 0))
    (:`then`
      (bind _output_get (set `self.Player` _asbp_player_controller))
      (bind _returnvalue (`|CreateWidget` "/Game/Game/Blueprints/AI/Dialogue_WB.Dialogue_WB_C" _output_get))
      (bind _output_get_2 (set `self.DialogueBox` _returnvalue))
      (`UserWidget.AddToViewport` _output_get_2 0)
      (`Widget.SetVisibility` _output_get_2 "Hidden"))
    (:`CastFailed`
      (`KismetSystemLibrary.PrintString` "Error Finding Player"))))

(event `self.PlayerDetector.OnComponentBeginOverlap`
  (params (OverlappedComponent :type "PrimitiveComponent Object Reference") (OtherActor :type "Actor Object Reference") (OtherComp :type "PrimitiveComponent Object Reference") (OtherBodyIndex :type Integer) (bFromSweep :type Boolean) (SweepResult :type "HitResult Structure (by ref)"))
  (cast `/Game/Unreal/Variant_Platforming/Blueprints/BP_PlatformingCharacter` OtherActor)
  (bind _asshop_creature_aic (cast `/Game/Game/Blueprints/AI/ShopCreature_AIC` (`self.GetController`)))
  (`/Game/Game/Blueprints/AI/ShopCreature_AIC.DisplayPopup` _asshop_creature_aic)
  (set `/Game/Game/Blueprints/Core/BP_PlayerController.NearbyChar` self (`self.Player`)))

(event `self.PlayerDetector.OnComponentEndOverlap`
  (params (OverlappedComponent :type "PrimitiveComponent Object Reference") (OtherActor :type "Actor Object Reference") (OtherComp :type "PrimitiveComponent Object Reference") (OtherBodyIndex :type Integer))
  (cast `/Game/Unreal/Variant_Platforming/Blueprints/BP_PlatformingCharacter` OtherActor)
  (bind _asshop_creature_aic (cast `/Game/Game/Blueprints/AI/ShopCreature_AIC` (`self.GetController`)))
  (`/Game/Game/Blueprints/AI/ShopCreature_AIC.HidePopup` _asshop_creature_aic)
  (set `/Game/Game/Blueprints/Core/BP_PlayerController.NearbyChar` null (`self.Player`))
  (`Widget.SetVisibility` (`self.DialogueBox`) "Hidden"))

(event `/Game/Game/Blueprints/AI/Dialogue_BPI.Talk`
  (if (`/Game/Game/Blueprints/Core/BP_PlayerController.HasQuest` (`self.Player`))
    (`self.SetDialogueBoxText` (`KismetTextLibrary.Conv_StringToText` (`KismetArrayLibrary.Array_Random` (`self.BasicDialogue`))))
    (else
      (bind _output_get (set `self.WantedItem` (`KismetMathLibrary.SelectString` "Carrots" "Wheat" (`KismetMathLibrary.RandomBool`))))
      (`self.SetDialogueBoxText` (`KismetTextLibrary.Conv_StringToText` (`KismetStringLibrary.Concat_StrStr` (`KismetArrayLibrary.Array_Random` (`self.QuestPrompts`)) _output_get)))
      (set `/Game/Game/Blueprints/Core/BP_PlayerController.HasQuest` true (`self.Player`)))))

(fn `SetDialogueBoxText`
  (params (TextToSet :type Text))
  (bind _dialoguebox (`self.DialogueBox`))
  (set `TextBlock.Text` TextToSet (`/Game/Game/Blueprints/AI/Dialogue_WB.DialogueText` _dialoguebox))
  (`Widget.SetVisibility` _dialoguebox "Visible"))

(fn `UserConstructionScript`
  (`parent.UserConstructionScript`))