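; Mother bird creature Blueprint that acts as a shop creature, toggling a popup when the player comes near.
; Its PlayerDetector overlap events filter for BP_PlatformingCharacter, then tell the ShopCreature_AIC controller to display or hide the popup.
; BeginPlay checks for BP_PlayerController and prints an error if the cast fails, but on success sets Player to None.
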(event `self.ReceiveBeginPlay`
  (`parent.ReceiveBeginPlay`)
  (cast `/Game/Game/Blueprints/Core/BP_PlayerController` (`GameplayStatics.GetPlayerController` 0)
    (:`then`
      (set `self.Player` null))
    (:`CastFailed`
      (`KismetSystemLibrary.PrintString` "Error Finding Player"))))

(event `self.PlayerDetector.OnComponentBeginOverlap`
  (params (OverlappedComponent :type "PrimitiveComponent Object Reference") (OtherActor :type "Actor Object Reference") (OtherComp :type "PrimitiveComponent Object Reference") (OtherBodyIndex :type Integer) (bFromSweep :type Boolean) (SweepResult :type "HitResult Structure (by ref)"))
  (cast `/Game/Unreal/Variant_Platforming/Blueprints/BP_PlatformingCharacter` OtherActor)
  (bind _asshop_creature_aic (cast `/Game/Game/Blueprints/AI/ShopCreature_AIC` (`self.GetController`)))
  (`/Game/Game/Blueprints/AI/ShopCreature_AIC.DisplayPopup` _asshop_creature_aic))

(event `self.PlayerDetector.OnComponentEndOverlap`
  (params (OverlappedComponent :type "PrimitiveComponent Object Reference") (OtherActor :type "Actor Object Reference") (OtherComp :type "PrimitiveComponent Object Reference") (OtherBodyIndex :type Integer))
  (cast `/Game/Unreal/Variant_Platforming/Blueprints/BP_PlatformingCharacter` OtherActor)
  (bind _asshop_creature_aic (cast `/Game/Game/Blueprints/AI/ShopCreature_AIC` (`self.GetController`)))
  (`/Game/Game/Blueprints/AI/ShopCreature_AIC.HidePopup` _asshop_creature_aic))

(fn `UserConstructionScript`
  (`parent.UserConstructionScript`))