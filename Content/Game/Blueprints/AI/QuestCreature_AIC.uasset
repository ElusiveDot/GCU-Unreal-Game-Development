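; AI controller for quest creatures that owns the button prompt telling the player how to interact.
; On BeginPlay, if the controlled pawn is a TalkableAnimal_BP, it creates the prompt widget for the first player controller and adds it to the viewport hidden.
; DisplayPopup and HidePopup events toggle the prompt's visibility when the widget is valid.
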(event `self.ReceiveBeginPlay`
  (`parent.ReceiveBeginPlay`)
  (cast `/Game/Game/Blueprints/AI/Pig_Creature/TalkableAnimal_BP` (`self.K2_GetPawn`))
  ; Creates the button prompt telling the user how to interact
  (bind _returnvalue (`|CreateWidget` "/Game/Game/HUD/ButtonPrompt_W.ButtonPrompt_W_C" (`GameplayStatics.GetPlayerController` 0)))
  (bind _output_get (set `self.Prompt` _returnvalue))
  (`UserWidget.AddToViewport` _output_get 0)
  (`Widget.SetVisibility` _output_get "Hidden"))

(event `DisplayPopup`
  (bind _prompt (`self.Prompt`))
  (`/Engine/EditorBlueprintResources/StandardMacros.IsValid` _prompt
    (:`Is Valid`
      (`Widget.SetVisibility` _prompt "Visible"))))

(event `HidePopup`
  (bind _prompt (`self.Prompt`))
  (`/Engine/EditorBlueprintResources/StandardMacros.IsValid` _prompt
    (:`Is Valid`
      (`Widget.SetVisibility` _prompt "Hidden"))))

(fn `UserConstructionScript`
  (`parent.UserConstructionScript`))