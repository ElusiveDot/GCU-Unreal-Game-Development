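; Grid inventory component that stores item objects in a map keyed by 2D coordinate within fixed dimensions.
; AddItem fills an empty slot or stacks onto the occupant, optionally falling back to FloodFillStack, which tries matching stacks, then scans the grid.
; BeginPlay spawns default items, splitting counts by max stack size.
; Items are removable by reference, coordinate or class; class removal only decrements counts, and events fire on slot placement and removal by reference.
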(event `self.ReceiveBeginPlay`
  (`self.SpawnDefaultItems`))

(event `self.ReceiveTick`
  (params (DeltaSeconds :type "Float (single-precision)")))

(fn `AddItem`
  (params (position :type "/Game/Game/Blueprints/Inventory/FItemCoordinate Structure") (itemObject :type "/Game/Game/Blueprints/Items/BP_ItemObject Object Reference") (floodFillStack :type Boolean))
  (returns (success :type Boolean))
  (locals (ObstructingObject :type "/Game/Game/Blueprints/Items/BP_ItemObject Object Reference"))
  (bind _position (`local.position`))
  (bind _itemobject (`local.itemObject`))
  (bind (_value _returnvalue) (`BlueprintMapLibrary.Map_Find` (`self.Inventory`) (`local.position`)))
  (if (`self.IsValidStorageCoordinate` position)
    (if _returnvalue
      (`/Engine/EditorBlueprintResources/StandardMacros.IsValid` _value
        (:`Is Valid`
          (bind _output_get (set `local.ObstructingObject` _value))
          (bind __allstacked (`/Game/Game/Blueprints/Items/BP_ItemObject.AddToStack` _output_get (`local.itemObject`)))
          (if __allstacked
            (return true)
            (else
              _)))
        (:`Is Not Valid`
          (`BlueprintMapLibrary.Map_Add` (`self.Inventory`) _position _itemobject :!label _label)
          (`self.OnItemAdded` _itemobject _position)
          (return true)))
      (else
        (goto _label))))
  (if (`local.floodFillStack`)
    (bind __success (`self.FloodFillStack` (`local.itemObject`)))
    (return __success)
    (else
      (return false))))

(fn `AddItemByClass`
  (params (position :type "/Game/Game/Blueprints/Inventory/FItemCoordinate Structure") (itemClass :type "/Game/Game/Blueprints/Items/BP_ItemObject Class Reference") (count :type Integer :default 1) (floodFillStack :type Boolean))
  (returns (success :type Boolean))
  (bind _returnvalue (`|GenericCreateObject` itemClass))
  (if (`KismetSystemLibrary.IsValid` _returnvalue)
    (`/Game/Game/Blueprints/Items/BP_ItemObject.SetCount` _returnvalue count)
    (bind _success (`self.AddItem` position _returnvalue floodFillStack))
    (return _success)))

(fn `CanAddOrStackItemAt`
  (params (_inItem :type "/Game/Game/Blueprints/Items/BP_ItemObject Object Reference") (_coordinate :type "/Game/Game/Blueprints/Inventory/FItemCoordinate Structure"))
  (returns (canAdd :type Boolean) (canStack :type Boolean))
  (bind (_value _returnvalue) (`BlueprintMapLibrary.Map_Find` (`self.Inventory`) _coordinate))
  (if (`self.IsValidStorageCoordinate` _coordinate)
    (if _returnvalue
      (return false (`/Game/Game/Blueprints/Items/BP_ItemObject.CanStack` _value _inItem))
      (else
        (return true true)))
    (else
      (return false false))))

(fn `FindItemAtCoordinate`
  (params (_coord :type "/Game/Game/Blueprints/Inventory/FItemCoordinate Structure"))
  (returns (item :type "/Game/Game/Blueprints/Items/BP_ItemObject Object Reference") (found :type Boolean))
  (bind (_value _returnvalue) (`BlueprintMapLibrary.Map_Find` (`self.Inventory`) _coord))
  (return _value _returnvalue))

(fn `FloodFillStack`
  (params (_target :type "/Game/Game/Blueprints/Items/BP_ItemObject Object Reference"))
  (returns (_success :type Boolean))
  (bind (_keypin _valuepin) (`|MapForEach` (`self.Inventory`))
    (:`then`
      (if (`/Game/Game/Blueprints/Items/BP_ItemObject.CanStack` _valuepin _target)
        (bind __allstacked (`/Game/Game/Blueprints/Items/BP_ItemObject.AddToStack` _valuepin (`local._target`)))
        (if __allstacked
          (return true))))
    (:`CompletedPin`
      (bind _coordinate (`self.LoopOverInventory`)
        (:`LoopBody`
          (bind _success (`self.AddItem` _coordinate (`local._target`)))
          (if _success
            (return true)))
        (:`Completed`
          (return false))))))

(fn `IsValidStorageCoordinate`
  (params (_inCoord :type "/Game/Game/Blueprints/Inventory/FItemCoordinate Structure"))
  (returns (valid :type Boolean))
  (bind (_inventorydimensions_x _inventorydimensions_y) (break `/Game/Game/Blueprints/Inventory/FItemCoordinate` (`self.InventoryDimensions`)))
  (return (not (or (< _inCoord_X_2_641D96804475351CCD4879B5B886D80A 0) (< _inCoord_Y_4_410E8CB04779D8E2334F26BC865BC8B0 0) (> _inCoord_X_2_641D96804475351CCD4879B5B886D80A (- _inventorydimensions_x 1)) (> _inCoord_Y_4_410E8CB04779D8E2334F26BC865BC8B0 (- _inventorydimensions_y 1))))))

(fn `RemoveItem`
  (params (_inItem :type "/Game/Game/Blueprints/Items/BP_ItemObject Object Reference"))
  (returns (success :type Boolean))
  (bind (_keypin _valuepin) (`|MapForEach` (`self.Inventory`))
    (:`then`
      (if (== _valuepin _inItem)
        (`BlueprintMapLibrary.Map_Remove` (`self.Inventory`) _keypin)
        (`self.OnItemRemoved`)
        (return true)))
    (:`CompletedPin`
      (return false))))

(fn `RemoveItemAtCoordinate`
  (params (_targetCoordinate :type "/Game/Game/Blueprints/Inventory/FItemCoordinate Structure"))
  (returns (success :type Boolean))
  (bind _returnvalue (`BlueprintMapLibrary.Map_Remove` (`self.Inventory`) _targetCoordinate))
  (return _returnvalue))

(fn `RemoveItemByClass`
  (params (itemClass :type "/Game/Game/Blueprints/Items/BP_ItemObject Soft Class Reference") (count :type Integer :default 1))
  (returns (success :type Boolean) (itemsRemoved :type Integer))
  (locals (HoldCount :type Integer :default 1))
  (bind _holdcount (`local.HoldCount`))
  (set `local.HoldCount` count)
  (bind _coordinate (`self.LoopOverInventory`)
    (:`LoopBody`
      (bind (_item _found) (`self.FindItemAtCoordinate` _coordinate))
      (if _found
        (`KismetSystemLibrary.IsObjectOfSoftClass` _item itemClass
          (:`True`
            (bind _count (`/Game/Game/Blueprints/Items/BP_ItemObject.Count` _item))
            (if (<= (`local.HoldCount`) _count)
              (`/Game/Game/Blueprints/Items/BP_ItemObject.SetCount` _item (- _count _holdcount))
              (return true (`local.HoldCount`))
              (else
                (set `local.HoldCount` (- _holdcount _count))
                (`/Game/Game/Blueprints/Items/BP_ItemObject.SetCount` _item 0)))))))
    (:`Completed`
      (return false (- (`local.count`) (`local.HoldCount`))))))

(fn `SpawnDefaultItems`
  (locals (CurrentStackCount :type Integer))
  (bind _currentstackcount (`local.CurrentStackCount`))
  (for _array_element (`self.DefaultItems`)
    (set `local.CurrentStackCount` (`.count_5_B3BBCAF24797F6B72F419A94856C565C` (break `/Game/Game/Blueprints/Inventory/FDefaultItemInformation` _array_element)))
    (bind _returnvalue (`|GenericCreateObject` (`.object_2_49BEC9C64E15477181BCAAB51BFB41CD` (break `/Game/Game/Blueprints/Inventory/FDefaultItemInformation` _array_element)) :!label _label))
    (bind _maxstackcount (`/Game/Game/Blueprints/Items/BP_ItemObject.MaxStackCount` _returnvalue))
    (bind _returnvalue_2 (- _currentstackcount _maxstackcount))
    (`/Game/Game/Blueprints/Items/BP_ItemObject.SetCount` _returnvalue (`KismetMathLibrary.SelectInt` _maxstackcount _currentstackcount (> _returnvalue_2 0)))
    (`self.AddItem` (break `/Game/Game/Blueprints/Inventory/FDefaultItemInformation` _array_element) _returnvalue true)
    (bind _output_get (set `local.CurrentStackCount` _returnvalue_2))
    (if (> _output_get 0)
      (goto _label))))