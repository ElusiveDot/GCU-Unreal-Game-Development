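; BP_PlayerController is the player controller that registers the farming, platforming and mouse-look input mappings and handles inventory, item-switch and talk input.
; The inventory action flip-flops the HUD's inventory through a message.
; Item switching equips the first-row inventory item at the input value's index through the pawn's equipment component, then highlights the HUD hotbar slot.
; Talk messages NearbyChar when it is valid and implements Dialogue_BPI.
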(event `self.ReceiveBeginPlay`
  (bind _returnvalue (subsystem `EnhancedInputLocalPlayerSubsystem`))
  (`EnhancedInputSubsystemInterface.AddMappingContext` _returnvalue "/Game/Game/Blueprints/Input/IMC_FarmInputMapping.IMC_FarmInputMapping" 0 (struct))
  (`EnhancedInputSubsystemInterface.AddMappingContext` _returnvalue "/Game/Unreal/Variant_Platforming/Input/IMC_Platforming.IMC_Platforming" 0 (struct))
  (`EnhancedInputSubsystemInterface.AddMappingContext` (subsystem `EnhancedInputLocalPlayerSubsystem`) "/Game/Unreal/Input/IMC_MouseLook.IMC_MouseLook" 0 (struct)))

(event `EnhancedInput|/Game/Game/Blueprints/Input/IA_Inventory`
  (params (ActionValue :type Boolean) (ElapsedSeconds :type "Float (double-precision)") (TriggeredSeconds :type "Float (double-precision)") (InputAction :type "InputAction Object Reference" :default "/Game/Game/Blueprints/Input/IA_Inventory.IA_Inventory"))
  (:`Triggered`
    (bind _isa (`/Engine/EditorBlueprintResources/StandardMacros.FlipFlop`)
      (:`A`
        _)
      (:`B`
        _))
    (message `/Game/Game/Blueprints/Inventory/IInventoryInterface.ToggleInventory` (`self.GetHUD`) _isa)))

(event `EnhancedInput|/Game/Game/Blueprints/Input/IA_SwitchItem`
  (params (ActionValue :type "Float (double-precision)") (ElapsedSeconds :type "Float (double-precision)") (TriggeredSeconds :type "Float (double-precision)") (InputAction :type "InputAction Object Reference" :default "/Game/Game/Blueprints/Input/IA_SwitchItem.IA_SwitchItem"))
  (bind _returnvalue (`self.GetComponentByClass` (`self.K2_GetPawn`) "/Game/Game/Blueprints/Equipment/BPC_EquipmentComponent.BPC_EquipmentComponent_C"))
  (:`Triggered`
    (`/Game/Game/Blueprints/Equipment/BPC_EquipmentComponent.TryEquipItemToSlot` :`self` _returnvalue :`_item` (`/Game/Game/Blueprints/Inventory/BPC_InventoryComponent.FindItemAtCoordinate` (`/Game/Game/Blueprints/Equipment/BPC_EquipmentComponent.GetInventory` _returnvalue) (make `/Game/Game/Blueprints/Inventory/FItemCoordinate` (- (`KismetMathLibrary.FFloor` ActionValue) 1))))
    (message `/Game/Game/Blueprints/Inventory/IInventoryInterface.SetHighlightedHotbar` (`self.GetHUD` (`GameplayStatics.GetPlayerController` 0)) ActionValue)))

(event `EnhancedInput|/Game/Game/Blueprints/AI/Talk_IA`
  (params (ActionValue :type Boolean) (ElapsedSeconds :type "Float (double-precision)") (TriggeredSeconds :type "Float (double-precision)") (InputAction :type "InputAction Object Reference" :default "/Game/Game/Blueprints/AI/Talk_IA.Talk_IA"))
  (bind _nearbychar (`self.NearbyChar`))
  (:`Started`
    (`/Engine/EditorBlueprintResources/StandardMacros.IsValid` _nearbychar
      (:`Is Valid`
        (if (`KismetSystemLibrary.DoesImplementInterface` _nearbychar "/Game/Game/Blueprints/AI/Dialogue_BPI.Dialogue_BPI_C")
          (message `/Game/Game/Blueprints/AI/Dialogue_BPI.Talk` _nearbychar))))))

(fn `UserConstructionScript`)