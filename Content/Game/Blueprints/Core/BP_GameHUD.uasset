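; BP_GameHUD owns the game's root UI widget, W_Base, creating it and adding it to the player screen at BeginPlay.
; Events bind a player inventory component to the inventory grid and both hotbar grids, each with slot range arguments.
; Toggling the inventory switches its visibility, input mode and mouse cursor together.
; Hotbar selection slides a highlight overlay along its canvas slot by a fixed step per one-based index.
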(event `self.ReceiveBeginPlay`
  (bind _returnvalue (`|CreateWidget` "/Game/Game/HUD/W_Base.W_Base_C"))
  (bind _output_get (set `self.Base` _returnvalue))
  (`UserWidget.AddToPlayerScreen` _output_get 0))

(event `/Game/Game/Blueprints/Inventory/IInventoryInterface.ToggleInventory`
  (params (`_show?` :type Boolean))
  (bind _returnvalue (`GameplayStatics.GetPlayerController` 0))
  (bind _w_inventory (`/Game/Game/HUD/W_Base.W_Inventory` (`self.Base`)))
  (if `_show?`
    (`Widget.SetVisibility` _w_inventory "Visible")
    (`WidgetBlueprintLibrary.SetInputMode_GameAndUIEx` _returnvalue _w_inventory "LockInFullscreen" false)
    (set `PlayerController.bShowMouseCursor` true _returnvalue)
    (else
      (`Widget.SetVisibility` _w_inventory "Collapsed")
      (`WidgetBlueprintLibrary.SetInputMode_GameOnly` _returnvalue)
      (set `PlayerController.bShowMouseCursor` false _returnvalue))))

(event `/Game/Game/Blueprints/Inventory/IInventoryInterface.AssignPlayerInventory`
  (params (_comp :type "/Game/Game/Blueprints/Inventory/BPC_InventoryComponent Object Reference"))
  (bind _w_inventory (`/Game/Game/HUD/W_Base.W_Inventory` (`self.Base`)))
  (`/Game/Game/HUD/Inventory/W_InventoryGrid.AddInventoryComponent` (`/Game/Game/HUD/W_Inventory.W_InventoryGrid` _w_inventory) _comp (make `/Game/Game/Blueprints/Inventory/FItemCoordinate` -1 -1) (make `/Game/Game/Blueprints/Inventory/FItemCoordinate` 1 -1))
  (`/Game/Game/HUD/Inventory/W_InventoryGrid.AddInventoryComponent` (`/Game/Game/HUD/W_Inventory.W_InventoryHotbarGrid` _w_inventory) _comp (make `/Game/Game/Blueprints/Inventory/FItemCoordinate` -1 -1) (make `/Game/Game/Blueprints/Inventory/FItemCoordinate` 0))
  (`/Game/Game/HUD/Inventory/W_InventoryGrid.AddInventoryComponent` (`/Game/Game/HUD/Inventory/W_Hotbar.W_InventoryGrid` (`/Game/Game/HUD/W_GameHUD.W_Hotbar` (`/Game/Game/HUD/W_Base.W_GameHUD` (`self.Base`)))) _comp (make `/Game/Game/Blueprints/Inventory/FItemCoordinate` -1 -1) (make `/Game/Game/Blueprints/Inventory/FItemCoordinate` 0)))

(event `/Game/Game/Blueprints/Inventory/IInventoryInterface.SetHighlightedHotbar`
  (params (_input :type "Float (double-precision)"))
  (`CanvasPanelSlot.SetPosition` (`WidgetLayoutLibrary.SlotAsCanvasSlot` (`/Game/Game/HUD/Inventory/W_Hotbar.HighlightOverlay` (`/Game/Game/HUD/W_GameHUD.W_Hotbar` (`/Game/Game/HUD/W_Base.W_GameHUD` (`self.Base`))))) (`KismetMathLibrary.MakeVector2D` (* (- _input 1.0) 100.0))))

(fn `UserConstructionScript`)