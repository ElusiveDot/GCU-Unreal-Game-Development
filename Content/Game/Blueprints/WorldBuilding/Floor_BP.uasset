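; Floor actor that builds a grid of ground tile meshes for world building, sized from Size and CubeSize.
; The construction script spawns a static mesh component per cell, all using the FlatGroundTypes mesh (grass, dirt or farmed), and stores each in FloorTiles by grid index.
; GetStoodOnTile looks up a position's tile by rounding its X/Y offset from the actor in half-CubeSize steps, unlike the full-CubeSize placement spacing.
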(fn `GetStoodOnTile`
  (params (Position :type "Vector Structure"))
  (returns (NewParam :type "StaticMeshComponent Object Reference"))
  (bind _returnvalue (`self.GetTransform`))
  (bind _returnvalue_2 (/ (`self.CubeSize`) 2.0))
  (bind (_value _returnvalue_3) (`BlueprintMapLibrary.Map_Find` (`self.FloorTiles`) (`KismetMathLibrary.MakeVector2D` (`KismetMathLibrary.Conv_IntToDouble` (`KismetMathLibrary.Round` (/ (- Position_X (.x (.location _returnvalue))) _returnvalue_2))) (`KismetMathLibrary.Conv_IntToDouble` (`KismetMathLibrary.Round` (/ (- Position_Y (.y (.location _returnvalue))) _returnvalue_2))))))
  (if _returnvalue_3
    (return _value)
    (else
      (return null))))

(fn `UserConstructionScript`
  (bind (_size_x _size_y) (`KismetMathLibrary.BreakVector` (`self.Size`)))
  (bind _cubesize (`self.CubeSize`))
  (bind (_gridsize_x _gridsize_y) (`KismetMathLibrary.BreakVector2D` (`self.GridSize`)))
  (`|ExecutionSequence`
    (:`then_0`
      (bind _output_get (set `self.Size` (`KismetMathLibrary.MakeVector` _size_x _size_y)))
      (set `self.GridSize` (`KismetMathLibrary.MakeVector2D` (`KismetMathLibrary.Conv_IntToDouble` (`KismetMathLibrary.Round` (/ (.x _output_get) _cubesize))) (`KismetMathLibrary.Conv_IntToDouble` (`KismetMathLibrary.Round` (/ (.y _output_get) _cubesize))))))
    (:`then_1`
      (for _index (range (+ (`KismetMathLibrary.FTrunc` _gridsize_x) 1))
        (for _index_2 (range (+ (`KismetMathLibrary.FTrunc` _gridsize_y) 1))
          (bind _returnvalue (`AddComponent|NODE_AddStaticMeshComponent-0` :`RelativeTransform` (`KismetMathLibrary.MakeTransform` (`KismetMathLibrary.MakeVector` (* _index (`self.CubeSize`)) (* _index_2 (`self.CubeSize`))))))
          (`BlueprintMapLibrary.Map_Add` (`self.FloorTiles`) (`KismetMathLibrary.MakeVector2D` (`KismetMathLibrary.Conv_IntToDouble` _index) (`KismetMathLibrary.Conv_IntToDouble` _index_2)) _returnvalue)
          (`StaticMeshComponent.SetStaticMesh` _returnvalue (select `/Game/Game/Blueprints/WorldBuilding/HorizontalGroundTypes` (`self.FlatGroundTypes`) :`NewEnumerator0` "/Game/Fab/GameDev_Starter_Kit_-_Farming__Free_Edition_/3D_Tile_Ground_01/StaticMeshes/3D_Tile_Ground_01.3D_Tile_Ground_01" :`NewEnumerator2` "/Game/Fab/GameDev_Starter_Kit_-_Farming__Free_Edition_/3D_Tile_Ground_02/StaticMeshes/3D_Tile_Ground_02.3D_Tile_Ground_02" :`NewEnumerator4` "/Game/Fab/GameDev_Starter_Kit_-_Farming__Free_Edition_/3D_Tile_Ground_03/StaticMeshes/3D_Tile_Ground_03.3D_Tile_Ground_03" :`NewEnumerator6` "/Game/Fab/GameDev_Starter_Kit_-_Farming__Free_Edition_/3D_Tile_Ground_04/StaticMeshes/3D_Tile_Ground_04.3D_Tile_Ground_04" :`NewEnumerator8` "/Game/Fab/GameDev_Starter_Kit_-_Farming__Free_Edition_/3D_Tile_Ground_05/StaticMeshes/3D_Tile_Ground_05.3D_Tile_Ground_05" :`NewEnumerator11` "/Game/Fab/GameDev_Starter_Kit_-_Farming__Free_Edition_/3D_Tile_Farm_Field_01/StaticMeshes/3D_Tile_Farm_Field_01.3D_Tile_Farm_Field_01" :`NewEnumerator1` "/Game/Fab/GameDev_Starter_Kit_-_Farming__Free_Edition_/3D_Tile_Ground_01A/StaticMeshes/3D_Tile_Ground_01A.3D_Tile_Ground_01A" :`NewEnumerator3` "/Game/Fab/GameDev_Starter_Kit_-_Farming__Free_Edition_/3D_Tile_Ground_02A/StaticMeshes/3D_Tile_Ground_02A.3D_Tile_Ground_02A" :`NewEnumerator5` "/Game/Fab/GameDev_Starter_Kit_-_Farming__Free_Edition_/3D_Tile_Ground_03A/StaticMeshes/3D_Tile_Ground_03A.3D_Tile_Ground_03A" :`NewEnumerator7` "/Game/Fab/GameDev_Starter_Kit_-_Farming__Free_Edition_/3D_Tile_Ground_04A/StaticMeshes/3D_Tile_Ground_04A.3D_Tile_Ground_04A" :!type "StaticMesh Object Reference")))))))