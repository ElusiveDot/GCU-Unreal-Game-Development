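; Tile_BP is a world-building ground tile whose GrassLevel represents how far its grass is eaten or regrown.
; SetMesh maps GrassLevel to one of the ground or farm field static meshes on the Tile component.
; EatLevel raises and GrowLevel lowers the level one step, with HalfTile choosing the index bounds for full or "A" mesh variants.
; SetLevel assigns a level directly without bounds checks, and every change refreshes the mesh.
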(fn `EatLevel`
  (bind _grasslevel (`self.GrassLevel`))
  (if (`self.HalfTile`)
    (if (< _grasslevel 9)
      (set `self.GrassLevel` (+ _grasslevel 1) :!label _label)
      (`self.SetMesh`))
    (elif (< _grasslevel 5)
      (goto _label))))

(fn `GrowLevel`
  (bind _grasslevel (`self.GrassLevel`))
  (if (`self.HalfTile`)
    (if (> _grasslevel 6)
      (set `self.GrassLevel` (- _grasslevel 1) :!label _label)
      (`self.SetMesh`))
    (elif (> _grasslevel 0)
      (goto _label))))

(fn `SetLevel`
  (params (NewLevel :type Integer))
  (set `self.GrassLevel` NewLevel)
  (`self.SetMesh`))

(fn `SetMesh`
  (`StaticMeshComponent.SetStaticMesh` (`self.Tile`) (select `int` (`self.GrassLevel`) :`0` "/Game/Fab/GameDev_Starter_Kit_-_Farming__Free_Edition_/3D_Tile_Ground_01/StaticMeshes/3D_Tile_Ground_01.3D_Tile_Ground_01" :`1` "/Game/Fab/GameDev_Starter_Kit_-_Farming__Free_Edition_/3D_Tile_Ground_02/StaticMeshes/3D_Tile_Ground_02.3D_Tile_Ground_02" :`2` "/Game/Fab/GameDev_Starter_Kit_-_Farming__Free_Edition_/3D_Tile_Ground_03/StaticMeshes/3D_Tile_Ground_03.3D_Tile_Ground_03" :`3` "/Game/Fab/GameDev_Starter_Kit_-_Farming__Free_Edition_/3D_Tile_Ground_04/StaticMeshes/3D_Tile_Ground_04.3D_Tile_Ground_04" :`4` "/Game/Fab/GameDev_Starter_Kit_-_Farming__Free_Edition_/3D_Tile_Ground_05/StaticMeshes/3D_Tile_Ground_05.3D_Tile_Ground_05" :`5` "/Game/Fab/GameDev_Starter_Kit_-_Farming__Free_Edition_/3D_Tile_Farm_Field_01/StaticMeshes/3D_Tile_Farm_Field_01.3D_Tile_Farm_Field_01" :`6` "/Game/Fab/GameDev_Starter_Kit_-_Farming__Free_Edition_/3D_Tile_Ground_01A/StaticMeshes/3D_Tile_Ground_01A.3D_Tile_Ground_01A" :`7` "/Game/Fab/GameDev_Starter_Kit_-_Farming__Free_Edition_/3D_Tile_Ground_02A/StaticMeshes/3D_Tile_Ground_02A.3D_Tile_Ground_02A" :`8` "/Game/Fab/GameDev_Starter_Kit_-_Farming__Free_Edition_/3D_Tile_Ground_03A/StaticMeshes/3D_Tile_Ground_03A.3D_Tile_Ground_03A" :`9` "/Game/Fab/GameDev_Starter_Kit_-_Farming__Free_Edition_/3D_Tile_Ground_04A/StaticMeshes/3D_Tile_Ground_04A.3D_Tile_Ground_04A" :!type "StaticMesh Object Reference")))

(fn `UserConstructionScript`)