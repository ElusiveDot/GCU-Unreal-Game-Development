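; Actor component that tracks equipped items in a map from slot tag to item and spawned world actor.
; Equipping clears the slot, spawns an A_WorldItem and attaches it to the owner's skeletal mesh, always at hand_r, with the item's offset; unequipping destroys it.
; Slot eligibility uses gameplay tag queries.
; It requires a sibling inventory component, but its item-removed handler, default-equipment spawning and CanEquipItem are unfinished.
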(event `self.ReceiveTick`
  (params (DeltaSeconds :type "Float (single-precision)"))
  (bind (_item _world_item _found_) (`self.GetEquipmentInSlot` (struct :`TagName` "Equipment.RightHand"))))

(event `self.ReceiveBeginPlay`
  (add `/Game/Game/Blueprints/Inventory/BPC_InventoryComponent.OnItemRemoved` (`self.GetInventory`) (`|CreateDelegate` :!event `HandleItemRemoved`)))

(event `HandleItemRemoved`)

(fn `CanEquipItem`
  (`|MapForEach` (`self.Equipment`)))

(fn `CanEquipItemToSlot`
  (params (_item :type "/Game/Game/Blueprints/Items/BP_ItemObject Object Reference") (_slot :type "GameplayTag Structure"))
  (returns (allow :type Boolean))
  (`/Engine/EditorBlueprintResources/StandardMacros.IsValid` _item
    (:`Is Valid`
      (if (`BlueprintMapLibrary.Map_Contains` (`self.Equipment`) _slot)
        _
        (elif (`BlueprintGameplayTagLibrary.DoesContainerMatchTagQuery` (`/Game/Game/Blueprints/Items/BP_ItemObject.EquipmentSlots` _item) (`BlueprintGameplayTagLibrary.MakeGameplayTagQuery_MatchAnyTags` (`BlueprintGameplayTagLibrary.MakeGameplayTagContainerFromTag` _slot)))
          (return true))))))

(fn `GetEquipmentInSlot`
  (params (inSlot :type "GameplayTag Structure"))
  (returns (Item :type "/Game/Game/Blueprints/Items/BP_ItemObject Object Reference") (`World Item` :type "/Game/Game/Blueprints/Items/A_WorldItem Object Reference") (`found?` :type Boolean))
  (bind (_value _returnvalue) (`BlueprintMapLibrary.Map_Find` (`self.Equipment`) inSlot))
  (if _returnvalue
    (return (break `/Game/Game/Blueprints/Equipment/FEquipment` _value) (`.worldItem_9_ADD03894406921299EEF0897142A618D` (break `/Game/Game/Blueprints/Equipment/FEquipment` _value)) _returnvalue)
    (else
      (return null null _returnvalue))))

(fn `GetInventory`
  (returns (inventory :type "/Game/Game/Blueprints/Inventory/BPC_InventoryComponent Object Reference"))
  (bind _inventory (`self.Inventory`)
    (:`then`
      (return _inventory))
    (:`else`
      (set `self.Inventory` (`Actor.GetComponentByClass` (`self.GetOwner`) "/Game/Game/Blueprints/Inventory/BPC_InventoryComponent.BPC_InventoryComponent_C"))
      (bind _inventory_2 (`self.Inventory`)
        (:`then`
          (return _inventory_2))
        (:`else`
          (`KismetSystemLibrary.PrintString` "Equipment Component requires matching inventory component to function." true true (struct :`R` 1.0 :`A` 1.0) 20.0)
          (`KismetSystemLibrary.RaiseScriptError` "Equipment Component requires matching inventory component to function.")
          (return null))))))

(fn `Internal_EquipItem`
  (params (_item :type "/Game/Game/Blueprints/Items/BP_ItemObject Object Reference") (_slot :type "GameplayTag Structure"))
  (bind (_itemdisplayinfo_name _itemdisplayinfo_description _itemdisplayinfo_brushasset _itemdisplayinfo_staticmesh _itemdisplayinfo_equippedpositionoffset) (break `/Game/Game/Blueprints/Items/FItemDisplayInformation` (`/Game/Game/Blueprints/Items/BP_ItemObject.ItemDisplayInfo` _item)))
  (bind _returnvalue (`|SpawnActorFromClass` "/Game/Game/Blueprints/Items/A_WorldItem.A_WorldItem_C" (`KismetMathLibrary.MakeTransform` (0.0 0.0 0.0)) "Undefined" "MultiplyWithRoot" null _item null))
  (`BlueprintMapLibrary.Map_Add` (`self.Equipment`) _slot (make `/Game/Game/Blueprints/Equipment/FEquipment` _item _returnvalue))
  (`Actor.K2_AttachToComponent` _returnvalue (`Actor.GetComponentByClass` (`self.GetOwner`) "/Script/Engine.SkeletalMeshComponent") "hand_r" "SnapToTarget" "SnapToTarget" "SnapToTarget" true)
  (`Actor.K2_SetActorRelativeTransform` _returnvalue _itemdisplayinfo_equippedpositionoffset false false))

(fn `Internal_UnequipSlot`
  (params (_slot :type "GameplayTag Structure"))
  (bind _equipment (`self.Equipment`))
  (bind (_value _returnvalue) (`BlueprintMapLibrary.Map_Find` _equipment _slot))
  (if _returnvalue
    (`Actor.K2_DestroyActor` (`.worldItem_9_ADD03894406921299EEF0897142A618D` (break `/Game/Game/Blueprints/Equipment/FEquipment` _value)))
    (`BlueprintMapLibrary.Map_Remove` _equipment _slot)
    (else
      (`KismetSystemLibrary.PrintString` "WHAT HOW \n"))))

(fn `SpawnDefaultEquipment`
  (bind (_keypin _valuepin) (`|MapForEach` (`self.DEFAULT_EQUIPMENT`))
    (:`then`
      (if (`KismetSystemLibrary.IsValidClass` (`.object_2_49BEC9C64E15477181BCAAB51BFB41CD` (break `/Game/Game/Blueprints/Inventory/FDefaultItemInformation` (break `/Game/Game/Blueprints/Equipment/FDefaultEquipment` _valuepin))))
        _))))

(fn `TryEquipItemToSlot`
  (params (_item :type "/Game/Game/Blueprints/Items/BP_ItemObject Object Reference") (_slot :type "GameplayTag Structure"))
  (returns (success :type Boolean))
  (`/Engine/EditorBlueprintResources/StandardMacros.IsValid` _item
    (:`Is Valid`
      (if (`BlueprintMapLibrary.Map_Contains` (`self.Equipment`) _slot)
        (bind _success (`self.TryUnequipSlot` _slot))
        (if _success
          _
          (else
            (return false))))
      (`self.Internal_EquipItem` (`local._item`) (`local._slot`))
      (return false))
    (:`Is Not Valid`
      (bind _success_2 (`self.TryUnequipSlot` _slot))
      (return _success_2))))

(fn `TryUnequipItem`
  (params (_item :type "/Game/Game/Blueprints/Items/BP_ItemObject Object Reference"))
  (returns (success :type Boolean))
  (`/Engine/EditorBlueprintResources/StandardMacros.IsValid` _item
    (:`Is Valid`
      (bind (_keypin _valuepin) (`|MapForEach` (`self.Equipment`))
        (:`then`
          (if (== (break `/Game/Game/Blueprints/Equipment/FEquipment` _valuepin) (`local._item`))
            (bind _success (`self.TryUnequipSlot` _keypin))
            (return _success)))))))

(fn `TryUnequipSlot`
  (params (_slot :type "GameplayTag Structure"))
  (returns (success :type Boolean))
  (if (`.ReturnValue` (`BlueprintMapLibrary.Map_Find` (`self.Equipment`) _slot))
    (`self.Internal_UnequipSlot` _slot)
    (return true)
    (else
      (return true))))