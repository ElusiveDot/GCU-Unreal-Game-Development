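; Actor component that manages a tag-keyed set of actions, each pairing an action object with an animation.
; On BeginPlay it constructs each configured action set and instantiates its action classes with a reference back to the manager, storing them by tag.
; Execution is unfinished: TryExecuteAction only looks up the tag and attempts to cancel the current action, TryCancelAction always returns false, and InternalCancelAction is empty.
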(event `self.ReceiveBeginPlay`
  (for _array_element (`self.ACTION_SETS`)
    (`self.Internal_AddActionSet` _array_element)))

(fn `Internal_AddActionSet`
  (params (_actionSet :type "/Game/Game/Blueprints/Action/BP_ActionSetBase Class Reference"))
  (bind _returnvalue (`|GenericCreateObject` _actionSet))
  (bind (_keypin _valuepin) (`|MapForEach` (`/Game/Game/Blueprints/Action/BP_ActionSetBase.Actions` _returnvalue))
    (:`then`
      (bind _returnvalue_2 (`|GenericCreateObject` (break `/Game/Game/Blueprints/Action/FActionSetConfig` _valuepin) self))
      (`BlueprintMapLibrary.Map_Add` (`self.ActionSet`) _keypin (make `/Game/Game/Blueprints/Action/FActionSetInstance` _returnvalue_2 (`.Animation_5_B73CFE604BE93C84AF52D8A6C12A5602` (break `/Game/Game/Blueprints/Action/FActionSetConfig` _valuepin)))))))

(fn `Internal_CancelAction`)

(fn `TryCancelAction`
  (params (tag :type "GameplayTag Structure"))
  (returns (`success?` :type Boolean))
  (return false))

(fn `TryExecuteAction`
  (params (tag :type "GameplayTag Structure"))
  (returns (`success?` :type Boolean))
  (if (`.ReturnValue` (`BlueprintMapLibrary.Map_Find` (`self.ActionSet`) tag))
    (bind _success_ (`self.TryCancelAction` (`self.CurrentActionTag`)))
    (if (not _success_)
      (return false))
    (else
      (return false))))