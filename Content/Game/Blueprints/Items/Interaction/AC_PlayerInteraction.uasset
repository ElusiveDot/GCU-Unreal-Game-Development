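; Player interaction component that lets the owning Character interact with nearby actors implementing BPI_Interface.
; Capsule overlaps maintain an in-range list, whose last entry is the active interactable and gets a runtime-created screen-space WB_Interaction prompt.
; IA_Interact triggers Press interactables immediately.
; For Hold types, it binds a dispatcher that passes elapsed time to update widget progress against the interactable's hold duration, unbinding on release.
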(event `self.ReceiveBeginPlay`
  (bind _returnvalue (`self.GetOwner`))
  (bind _ascharacter (cast `Character` _returnvalue))
  (bind _capsulecomponent (`Character.CapsuleComponent` _ascharacter))
  (add `PrimitiveComponent.OnComponentBeginOverlap` _capsulecomponent (`|CreateDelegate` :!event `HandleCaspuleOverlapBegin`))
  (add `PrimitiveComponent.OnComponentEndOverlap` _capsulecomponent (`|CreateDelegate` :!event `HandleCaspuleOverlapEnd`))
  ; Widget Creation
  (bind _returnvalue_2 (`|AddComponentByClass` :`self` _returnvalue :`Class` "/Script/UMG.WidgetComponent" :`bManualAttachment` true))
  (`WidgetComponent.SetWidgetSpace` _returnvalue_2 "Screen")
  (`WidgetComponent.SetDrawSize` _returnvalue_2 (250.0 30.0))
  (set `self.InteractionWidgetComponent` _returnvalue_2))

(event `HandleCaspuleOverlapBegin`
  (params (OverlappedComponent :type "PrimitiveComponent Object Reference") (OtherActor :type "Actor Object Reference") (OtherComp :type "PrimitiveComponent Object Reference") (OtherBodyIndex :type Integer) (bFromSweep :type Boolean) (SweepResult :type "HitResult Structure (by ref)"))
  ; Pickup and Remove
  (if (`KismetSystemLibrary.DoesImplementInterface` OtherActor "/Game/Game/Blueprints/Items/Interaction/BPI_Interface.BPI_Interface_C")
    (`KismetArrayLibrary.Array_AddUnique` (`self.InteractablesInRange`) OtherActor)
    (`self.RenderInteractionWidget`)))

(event `EnhancedInput|/Game/Unreal/Variant_Platforming/Input/Actions/IA_Interact`
  (params (ActionValue :type Boolean) (ElapsedSeconds :type "Float (double-precision)") (TriggeredSeconds :type "Float (double-precision)") (InputAction :type "InputAction Object Reference" :default "/Game/Unreal/Variant_Platforming/Input/Actions/IA_Interact.IA_Interact"))
  ; Interact & Widgets
  (:`Started`
    (`self.InteractBegin`))
  (:`Ongoing`
    (`self.OnInteractionPress` ElapsedSeconds))
  (:`Canceled`
    (clear `self.OnInteractionPress` :!label _label)
    (bind _interactionwidgetref (`self.InteractionWidgetREF`)
      (:`then`
        (`/Game/Game/Blueprints/Items/Interaction/WB_Interaction.SetProgressPerecent` _interactionwidgetref 0.0))
      (:`else`)))
  (:`Completed`
    (goto _label)))

(event `InteractBegin`
  (bind _output (`self.GetActiveInteractable`))
  ; Interact & Widgets
  (`/Engine/EditorBlueprintResources/StandardMacros.IsValid` _output
    (:`Is Valid`
      (bind _type (message `/Game/Game/Blueprints/Items/Interaction/BPI_Interface.InteractionType` _output))
      (switch `/Game/Game/Blueprints/Items/Interaction/Enum_InteractionType` _type
        (:`NewEnumerator0`
          (`self.InteractWithActiveInteractable`))
        (:`NewEnumerator1`
          (add `self.OnInteractionPress` (delegate `OnInteractionOngoing`)))))))

(event `HandleCaspuleOverlapEnd`
  (params (OverlappedComponent :type "PrimitiveComponent Object Reference") (OtherActor :type "Actor Object Reference") (OtherComp :type "PrimitiveComponent Object Reference") (OtherBodyIndex :type Integer))
  ; Pickup and Remove
  (if (`KismetSystemLibrary.DoesImplementInterface` OtherActor "/Game/Game/Blueprints/Items/Interaction/BPI_Interface.BPI_Interface_C")
    (`KismetArrayLibrary.Array_RemoveItem` (`self.InteractablesInRange`) OtherActor)
    (`self.RenderInteractionWidget`)))

(event `OnInteractionOngoing` :!signature `self.OnInteractionPress`
  (params (ElapsedSeconds :type "Float (double-precision)"))
  (bind _output (`self.GetActiveInteractable`))
  ; Interact & Widgets
  (`/Engine/EditorBlueprintResources/StandardMacros.IsValid` _output
    (:`Is Valid`
      (bind _duration (message `/Game/Game/Blueprints/Items/Interaction/BPI_Interface.GetHoldDuration` _output))
      (bind _interactionwidgetref (`self.InteractionWidgetREF`)
        (:`then`
          (`/Game/Game/Blueprints/Items/Interaction/WB_Interaction.SetProgressPerecent` _interactionwidgetref (/ ElapsedSeconds _duration)))
        (:`else`
          _))
      (if (>= 0.0 _duration)
        (`self.InteractWithActiveInteractable`)
        (remove `self.OnInteractionPress` (delegate `OnInteractionOngoing`))))))

(event `InteractWithActiveInteractable`
  (bind _output (`self.GetActiveInteractable`))
  ; Interact & Widgets
  (if (`KismetArrayLibrary.Array_IsNotEmpty` (`self.InteractablesInRange`))
    (`/Engine/EditorBlueprintResources/StandardMacros.IsValid` _output
      (:`Is Valid`
        (if (`KismetSystemLibrary.DoesImplementInterface` _output "/Game/Game/Blueprints/Items/Interaction/BPI_Interface.BPI_Interface_C")
          (message `/Game/Game/Blueprints/Items/Interaction/BPI_Interface.Interaction` _output (`self.GetOwner`)))))))

(fn `GetActiveInteractable`
  (returns (Output :type "Actor Object Reference"))
  (bind _interactablesinrange (`self.InteractablesInRange`))
  (return (`|GetArrayItem` _interactablesinrange (`KismetArrayLibrary.Array_LastIndex` _interactablesinrange))))

(fn `RenderInteractionWidget`
  (bind _output (`self.GetActiveInteractable`))
  (`/Engine/EditorBlueprintResources/StandardMacros.IsValid` _output
    (:`Is Valid`
      (bind _type (message `/Game/Game/Blueprints/Items/Interaction/BPI_Interface.InteractionType` _output))
      (bind _returnvalue (`|CreateWidget` "/Game/Game/Blueprints/Items/Interaction/WB_Interaction.WB_Interaction_C" null _type))
      (`WidgetComponent.SetWidget` (`self.InteractionWidgetComponent`) _returnvalue)
      (`SceneComponent.K2_SetWorldLocation` (`self.InteractionWidgetComponent`) (`Actor.K2_GetActorLocation` (`self.GetActiveInteractable`)) false false))
    (:`Is Not Valid`
      (`WidgetComponent.SetWidget` (`self.InteractionWidgetComponent`) null))))