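; BP_ItemObject represents a stackable inventory item with a gameplay tag, count, maximum stack size and world item reference.
; AddToStack moves as much as fits from an item with an exactly matching tag and reports whether that source is emptied.
; RemoveFromStack clamps removal and reports the amount removed and whether the request was fully met.
; Both route through SetCount, which fires stack updated and, at zero or below, stack emptied events.
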(fn `AddToStack`
  (params (_otherItem :type "/Game/Game/Blueprints/Items/BP_ItemObject Object Reference"))
  (returns (_allStacked :type Boolean))
  (locals (HoldOtherItemCount :type Integer :default 0))
  (bind _count (`self.Count`))
  (bind __otheritem (`local._otherItem`))
  (if (`self.CanStack` _otherItem)
    (`|ExecutionSequence`
      (:`then_0`
        (bind _output_get (set `local.HoldOtherItemCount` (`/Game/Game/Blueprints/Items/BP_ItemObject.Count` __otheritem)))
        (bind _returnvalue (`KismetMathLibrary.Clamp` (- (`self.MaxStackCount`) _count) 0 _output_get))
        (`self.SetCount` __otheritem (- _output_get _returnvalue))
        (`self.SetCount` (+ _count _returnvalue)))
      (:`then_1`
        (return (<= (`/Game/Game/Blueprints/Items/BP_ItemObject.Count` (`local._otherItem`)) 0))))
    (else
      (return false))))

(fn `CanStack`
  (params (_otherObject :type "/Game/Game/Blueprints/Items/BP_ItemObject Object Reference"))
  (returns (_canStack :type Boolean))
  (return (and (`BlueprintGameplayTagLibrary.MatchesTag` (`/Game/Game/Blueprints/Items/BP_ItemObject.ItemTag` _otherObject) (`self.ItemTag`) true) (< (`self.Count`) (`self.MaxStackCount`)))))

(fn `GetWorldItem`
  (returns (_outItem :type "/Game/Game/Blueprints/Items/A_WorldItem Soft Class Reference"))
  (return (`self.WorldItem`)))

(fn `RemoveFromStack`
  (params (_removeCount :type Integer))
  (returns (_removed :type Integer) (_resolved :type Boolean))
  (bind _returnvalue (`KismetMathLibrary.Clamp` _removeCount 0 (`self.Count`)))
  (`self.SetCount` (- (`self.Count`) _returnvalue))
  (return _returnvalue (== _removeCount _returnvalue)))

(fn `SetCount`
  (params (_newCount :type Integer))
  (bind _output_get (set `self.Count` _newCount))
  (`self.OnStackUpdated` self)
  (if (<= _output_get 0)
    (`self.OnStackEmptied` self)))