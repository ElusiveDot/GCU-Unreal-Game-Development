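; Farmable crop plot that, on player interaction, grows a plant through staged meshes and then yields a carrot world item.
; ExecuteGrowth swaps Plant meshes between delays, with GrowTime overridden if the player's WateringCan flag is set.
; At harvest it hides the plant, spawns the item and destroys its collision.
; Interaction also checks overlapping plots, but the growth call follows the empty loop, reaching only the last element.
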(event `ExecuteGrowth`
  (bind _plant (`self.Plant`))
  (bind _plant_2 (`self.Plant`))
  (bind _plant_3 (`self.Plant`))
  (bind _asbp_platforming_character (cast `/Game/Unreal/Variant_Platforming/Blueprints/BP_PlatformingCharacter` (`GameplayStatics.GetPlayerCharacter` 0)))
  (`KismetSystemLibrary.PrintString` "Seed found")
  (bind _returnvalue (`StaticMeshComponent.SetStaticMesh` _plant_2 (`|GetArrayItem` (`self.PlantMeshes`) 1)))
  (if _returnvalue
    (`SceneComponent.SetVisibility` _plant_2 true false)
    (`KismetSystemLibrary.PrintString` "Success")
    (if (== (`/Game/Unreal/Variant_Platforming/Blueprints/BP_PlatformingCharacter.WateringCan?` _asbp_platforming_character) true)
      (bind _output_get (set `self.Grow Time` 15.0))
      (`KismetSystemLibrary.Delay` _output_get)
      (else
        (`KismetSystemLibrary.Delay` (`self.Grow Time`))))
    (bind _returnvalue_2 (`StaticMeshComponent.SetStaticMesh` _plant (`|GetArrayItem` (`self.PlantMeshes`) 2)))
    (`SceneComponent.SetVisibility` _plant true false)
    (if _returnvalue_2
      (bind _asbp_platforming_character_2 (cast `/Game/Unreal/Variant_Platforming/Blueprints/BP_PlatformingCharacter` (`GameplayStatics.GetPlayerCharacter` 0)))
      (if (== (`/Game/Unreal/Variant_Platforming/Blueprints/BP_PlatformingCharacter.WateringCan?` _asbp_platforming_character_2) true)
        (bind _output_get_2 (set `self.Grow Time` 15.0))
        (`KismetSystemLibrary.Delay` _output_get_2)
        (else
          (`KismetSystemLibrary.Delay` (`self.Grow Time`))))
      (`SceneComponent.SetVisibility` _plant_3 false false)
      (`|SpawnActorFromClass` "/Game/Game/Blueprints/Items/A_WorldItem.A_WorldItem_C" (`KismetMathLibrary.MakeTransform` (`SceneComponent.K2_GetComponentLocation` _plant_3)) "Undefined" "MultiplyWithRoot" null null "NewEnumerator1" 10.0 "/Game/Game/Blueprints/Items/Items/BP_Carrot.BP_Carrot_C" "/Game/Game/Art/Items/S_Carrot.S_Carrot" null)
      (`ActorComponent.K2_DestroyComponent` (`self.Collision`)))
    (else
      (`KismetSystemLibrary.PrintString` "No Pant"))))

(event `/Game/Game/Blueprints/Items/Interaction/BPI_Interface.Interaction`
  (params (InteractorNewParam :type "Actor Object Reference"))
  (`|ExecutionSequence`
    (:`then_0`
      (`self.ExecuteGrowth`))
    (:`then_1`
      (for _array_element (`PrimitiveComponent.GetOverlappingActors` (`self.Detection`) "Farmable_BPC_C")
        _)
      (bind _asfarmable_bpc (cast `/Game/Game/Blueprints/Items/Farmable_BPC` _array_element))
      (`self.ExecuteGrowth` _asfarmable_bpc))))

(fn `GetHoldDuration`
  (returns (Duration :type "Float (double-precision)"))
  (return 0.0))

(fn `InteractionType`
  (returns (Type :type "/Game/Game/Blueprints/Items/Interaction/Enum_InteractionType Enum"))
  (return "NewEnumerator0"))

(fn `UserConstructionScript`)